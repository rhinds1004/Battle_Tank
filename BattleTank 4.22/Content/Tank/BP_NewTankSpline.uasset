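; Player tank pawn with gimbal camera, toggleable third-person view, health bar widget and animated spline tread.
; Input drives TankMovement and TankAiming components for driving and firing, and rotates the camera gimbal and spring arm.
; Construction Script lays spline mesh segments along Spline2 at the Right Track socket, alternating materials and caching their distances.
; Tick slides segments along the spline by TrackLeftLinVel, wrapping at its length to loop the tread.
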(event EventBeginPlay
  (Class|TankAimingComponent|Initialize (Variables|Default|GetTankAiming) (Variables|Default|GetTankBarrel) (Variables|Default|GetTurret))
  (Class|TankMovementComponent|Initialize (Variables|Default|GetTankMovement) (Variables|Default|GetLTankTrack) (Variables|Default|GetRTankTrack))
  (CallFunction|InitializeHealthBarWidget))

(event Collision|EventActorBeginOverlap
  (params (OtherActor :type Actor%20Object%20Reference)))

(event EventTick
  (params (DeltaSeconds :type Float%20%28single-precision%29))
  (CallFunction|MoveTreads))

(event Input|ActionEvents|InputActionToggle3rdPersonCamera
  (params (Key :type Key%20Structure))
  ;[1 1 1] Toggles between first and 3rd person view.
  (:Pressed
    (Components|Activation|ToggleActive (Variables|Default|Get3rd%20person))))

(event Input|KeyboardEvents|L
  (params (Key :type Key%20Structure)))

(event Input|AxisEvents|InputAxisAimAzimuth
  (params (AxisValue :type Float%20%28single-precision%29))
  (Transformation|AddLocalRotation (Variables|Default|GetAzimuth%20Gimbal) (Math|Rotator|MakeRotator 0.0 0.0 (* AxisValue (Utilities|Time|GetWorldDeltaSeconds) 1e+02)) false false))

(event Input|AxisEvents|InputAxisAimElevation
  (params (AxisValue :type Float%20%28single-precision%29))
  (Transformation|AddLocalRotation (Variables|Default|GetSpringArm) (Math|Rotator|MakeRotator 0.0 (* AxisValue (Utilities|Time|GetWorldDeltaSeconds) 1e+02) 0.0) false false))

(event Input|GamepadEvents|GamepadLeftX
  (params (AxisValue :type Float%20%28single-precision%29))
  (Class|TankMovementComponent|IntendMoveRight (Variables|Default|GetTankMovement) AxisValue))

(event Input|GamepadEvents|GamepadLeftY
  (params (AxisValue :type Float%20%28single-precision%29))
  (Class|TankMovementComponent|IntendMoveForward (Variables|Default|GetTankMovement) AxisValue))

(event Input|GamepadEvents|GamepadFaceButtonBottom
  (params (Key :type Key%20Structure))
  (:Pressed
    (Class|TankAimingComponent|Fire (Variables|Default|GetTankAiming))))

(fn ConstructionScript
  (bind _spline2 (Variables|Default|GetSpline2))
  (bind _returnvalue (Spline|GetSplineLength _spline2))
  (while (<= (Variables|Default|GetCurrDist) _returnvalue)
    (bind _returnvalue_2 (AddComponent|AddSplineMeshComponent false))
    (Collision|SetCollisionEnabled _returnvalue_2 "QueryAndPhysics")
    (Transformation|AttachComponentToComponent _returnvalue_2 (Variables|Default|GetTank) "Right Track" "KeepRelative" "KeepRelative" "KeepRelative" true)
    (SplineMesh|SetStartandEnd _returnvalue_2 (Spline|GetLocationatDistanceAlongSpline _spline2 (Variables|Default|GetPrevDist) "Local") (Math|Vector|Normalize (Spline|GetTangentatDistanceAlongSpline _spline2 (Variables|Default|GetPrevDist) "Local")) (Spline|GetLocationatDistanceAlongSpline _spline2 (Variables|Default|GetCurrDist) "Local") (Math|Vector|Normalize (Spline|GetTangentatDistanceAlongSpline _spline2 (Variables|Default|GetCurrDist) "Local")) true :!class /Script/Engine.SplineMeshComponent)
    (Components|StaticMesh|SetStaticMesh _returnvalue_2 "/Game/Meshes/TreadSegment.TreadSegment")
    (bind _returnvalue_3 (Utilities|Array|Add (Variables|Default|GetTreadMeshes) _returnvalue_2))
    (Utilities|Array|Add (Variables|Default|Get2dArray) (Utilities|Struct|Make2dArray (Utilities|Array|MakeArray (Variables|Default|GetPrevDist) (Variables|Default|GetCurrDist))))
    (Variables|Default|SetPrevDist (Variables|Default|GetCurrDist))
    (Variables|Default|SetCurrDist (+ (Variables|Default|GetCurrDist) 2e+01))
    (Transformation|SetWorldTransform (Utilities|Array|Get(acopy) (Variables|Default|GetTreadMeshes) _returnvalue_3) (Math|Transform|MakeTransform (+ (.location (Transformation|GetWorldTransform (Utilities|Array|Get(acopy) (Variables|Default|GetTreadMeshes) _returnvalue_3))) "0.100000,0.100000,0.100000") (.rotation (Transformation|GetWorldTransform (Utilities|Array|Get(acopy) (Variables|Default|GetTreadMeshes) _returnvalue_3))) (.scale (Transformation|GetWorldTransform (Utilities|Array|Get(acopy) (Variables|Default|GetTreadMeshes) _returnvalue_3)))) false false)
    (Transformation|SetWorldTransform (Utilities|Array|Get(acopy) (Variables|Default|GetTreadMeshes) _returnvalue_3) (Math|Transform|MakeTransform (- (.location (Transformation|GetWorldTransform (Utilities|Array|Get(acopy) (Variables|Default|GetTreadMeshes) _returnvalue_3))) "0.100000,0.100000,0.100000") (.rotation (Transformation|GetWorldTransform (Utilities|Array|Get(acopy) (Variables|Default|GetTreadMeshes) _returnvalue_3))) (.scale (Transformation|GetWorldTransform (Utilities|Array|Get(acopy) (Variables|Default|GetTreadMeshes) _returnvalue_3)))) false false)
    (switch int (Math|Integer|%(Integer) _returnvalue_3 2)
      (:0
        (Rendering|Material|SetMaterial (Utilities|Array|Get(acopy) (Variables|Default|GetTreadMeshes) _returnvalue_3) 0 "/Engine/EngineDebugMaterials/VertexColorViewMode_RedOnly.VertexColorViewMode_RedOnly"))))
  (if (not (Math|Float|NearlyEqual(Float) (- _returnvalue (Variables|Default|GetCurrDist)) 0.0 1e-06))
    (bind _returnvalue_4 (AddComponent|AddSplineMeshComponent false))
    (Collision|SetCollisionEnabled _returnvalue_4 "QueryAndPhysics")
    (Transformation|AttachComponentToComponent _returnvalue_4 (Variables|Default|GetTank) "Right Track" "KeepRelative" "KeepRelative" "KeepRelative" true)
    (SplineMesh|SetStartandEnd _returnvalue_4 (Spline|GetLocationatDistanceAlongSpline _spline2 (Variables|Default|GetPrevDist) "Local") (Math|Vector|Normalize (Spline|GetTangentatDistanceAlongSpline _spline2 (Variables|Default|GetPrevDist) "Local")) (Spline|GetLocationatDistanceAlongSpline _spline2 (Variables|Default|GetCurrDist) "Local") (Math|Vector|Normalize (Spline|GetTangentatDistanceAlongSpline _spline2 (Variables|Default|GetCurrDist) "Local")) true :!class /Script/Engine.SplineMeshComponent)
    (Components|StaticMesh|SetStaticMesh _returnvalue_4 "/Game/Meshes/TreadSegment.TreadSegment")
    (bind _returnvalue_5 (Utilities|Array|Add (Variables|Default|GetTreadMeshes) _returnvalue_4))
    (Utilities|Array|Add (Variables|Default|Get2dArray) (Utilities|Struct|Make2dArray (Utilities|Array|MakeArray (Variables|Default|GetPrevDist) (Variables|Default|GetCurrDist))))
    (Variables|Default|SetPrevDist (Variables|Default|GetCurrDist))
    (Variables|Default|SetCurrDist (+ (Variables|Default|GetCurrDist) 2e+01))
    (Transformation|SetWorldTransform (Utilities|Array|Get(acopy) (Variables|Default|GetTreadMeshes) _returnvalue_5) (Math|Transform|MakeTransform (+ (.location (Transformation|GetWorldTransform (Utilities|Array|Get(acopy) (Variables|Default|GetTreadMeshes) _returnvalue_5))) "0.100000,0.100000,0.100000") (.rotation (Transformation|GetWorldTransform (Utilities|Array|Get(acopy) (Variables|Default|GetTreadMeshes) _returnvalue_5))) (.scale (Transformation|GetWorldTransform (Utilities|Array|Get(acopy) (Variables|Default|GetTreadMeshes) _returnvalue_5)))) false false)
    (Transformation|SetWorldTransform (Utilities|Array|Get(acopy) (Variables|Default|GetTreadMeshes) _returnvalue_5) (Math|Transform|MakeTransform (- (.location (Transformation|GetWorldTransform (Utilities|Array|Get(acopy) (Variables|Default|GetTreadMeshes) _returnvalue_5))) "0.100000,0.100000,0.100000") (.rotation (Transformation|GetWorldTransform (Utilities|Array|Get(acopy) (Variables|Default|GetTreadMeshes) _returnvalue_5))) (.scale (Transformation|GetWorldTransform (Utilities|Array|Get(acopy) (Variables|Default|GetTreadMeshes) _returnvalue_5)))) false false)
    (switch int (Math|Integer|%(Integer) _returnvalue_5 2)
      (:0
        (Rendering|Material|SetMaterial (Utilities|Array|Get(acopy) (Variables|Default|GetTreadMeshes) _returnvalue_5) 0 "/Engine/EngineDebugMaterials/VertexColorViewMode_RedOnly.VertexColorViewMode_RedOnly")))))

(fn InitializeHealthBarWidget
  (bind _asbp_health_bar (Utilities|Casting|CastToBP_HealthBar (UserInterface|GetUserWidgetObject (Variables|Default|GetWidget))))
  (Variables|/Game/UI/BP_HealthBar.BP_HealthBar_C|SetMyTank _asbp_health_bar self)
  (return))

(fn MoveTreads
  (bind _returnvalue (Utilities|Time|GetWorldDeltaSeconds))
  (bind _spline2 (Variables|Default|GetSpline2))
  (bind _spline2_2 (Variables|Default|GetSpline2))
  (bind _trackleftlinvel (Variables|Default|GetTrackLeftLinVel))
  (bind _returnvalue_2 (Spline|GetSplineLength _spline2_2))
  (bind _returnvalue_3 (* _trackleftlinvel _returnvalue))
  (for _index (range 0 (- (Utilities|Array|Length (Variables|Default|GetTreadMeshes)) 1))
    (SplineMesh|SetStartandEnd (Utilities|Array|Get(acopy) (Variables|Default|GetTreadMeshes) _index) (Spline|GetLocationatDistanceAlongSpline _spline2 (Math|Float|%(Float) (+ (Utilities|Array|Get(acopy) (Utilities|Struct|Break2dArray (Utilities|Array|Get(acopy) (Variables|Default|Get2dArray) _index))) _returnvalue_3) _returnvalue_2) "Local") (Math|Vector|Normalize (Spline|GetTangentatDistanceAlongSpline _spline2 (Math|Float|%(Float) (+ (Utilities|Array|Get(acopy) (Utilities|Struct|Break2dArray (Utilities|Array|Get(acopy) (Variables|Default|Get2dArray) _index))) _returnvalue_3) _returnvalue_2) "Local")) (Spline|GetLocationatDistanceAlongSpline _spline2 (Math|Float|%(Float) (+ (Utilities|Array|Get(acopy) (Utilities|Struct|Break2dArray (Utilities|Array|Get(acopy) (Variables|Default|Get2dArray) _index)) 1) _returnvalue_3) _returnvalue_2) "Local") (Math|Vector|Normalize (Spline|GetTangentatDistanceAlongSpline _spline2 (Math|Float|%(Float) (+ (Utilities|Array|Get(acopy) (Utilities|Struct|Break2dArray (Utilities|Array|Get(acopy) (Variables|Default|Get2dArray) _index)) 1) _returnvalue_3) _returnvalue_2) "Local")) true :!class /Script/Engine.SplineMeshComponent)
    (|SetBy-RefVar (Utilities|Array|Get(acopy) (Utilities|Struct|Break2dArray (Utilities|Array|Get(acopy) (Variables|Default|Get2dArray) _index))) (Math|Float|%(Float) (+ (Utilities|Array|Get(acopy) (Utilities|Struct|Break2dArray (Utilities|Array|Get(acopy) (Variables|Default|Get2dArray) _index))) _returnvalue_3) _returnvalue_2))
    (|SetBy-RefVar (Utilities|Array|Get(acopy) (Utilities|Struct|Break2dArray (Utilities|Array|Get(acopy) (Variables|Default|Get2dArray) _index)) 1) (Math|Float|%(Float) (+ (Utilities|Array|Get(acopy) (Utilities|Struct|Break2dArray (Utilities|Array|Get(acopy) (Variables|Default|Get2dArray) _index)) 1) _returnvalue_3) _returnvalue_2))))