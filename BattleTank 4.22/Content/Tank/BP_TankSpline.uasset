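; Player tank pawn that drives, aims a gimbal camera, fires and toggles third-person view, delegating to TankMovement and TankAiming components.
; BeginPlay initializes both components and links the health bar widget to the tank.
; The construction script builds spline meshes along Spline1, tinting alternate segments as an apparent tread experiment.
; Pressing L offsets segments one point using the first point's tangent; Movetreads, a per-point-tangent variant with debug prints, is uncalled here.
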(event EventBeginPlay
  (Class|TankAimingComponent|Initialize (Variables|Default|GetTankAiming) (Variables|Default|GetTankBarrel) (Variables|Default|GetTurret))
  (Class|TankMovementComponent|Initialize (Variables|Default|GetTankMovement) (Variables|Default|GetLTankTrack) (Variables|Default|GetRTankTrack))
  (CallFunction|InitializeHealthBarWidget))

(event Collision|EventActorBeginOverlap
  (params (OtherActor :type Actor%20Object%20Reference)))

(event EventTick
  (params (DeltaSeconds :type Float%20%28single-precision%29)))

(event Input|ActionEvents|InputActionToggle3rdPersonCamera
  (params (Key :type Key%20Structure))
  ;[1 1 1] Toggles between first and 3rd person view.
  (:Pressed
    (Components|Activation|ToggleActive (Variables|Default|Get3rd%20person))))

(event Input|KeyboardEvents|L
  (params (Key :type Key%20Structure))
  (bind _spline1 (Variables|Default|GetSpline1))
  (:Pressed
    (Variables|Default|SetLastIndex (- (Spline|GetNumberOfSplinePoints (Variables|Default|GetSpline1)) 1))
    (for _index (range 0 (Variables|Default|GetLastIndex))
      (SplineMesh|SetStartandEnd (Utilities|Array|Get(acopy) (Variables|Default|GetMeshes) _index) (Spline|GetLocationatSplinePoint _spline1 (+ _index 1) "Local") (Spline|GetTangentatSplinePoint _spline1 0 "Local") (Spline|GetLocationatSplinePoint _spline1 (+ _index 2) "Local") (Spline|GetTangentatSplinePoint _spline1 0 "Local") true :!class /Script/Engine.SplineMeshComponent))))

(event Input|AxisEvents|InputAxisAimAzimuth
  (params (AxisValue :type Float%20%28single-precision%29))
  (Transformation|AddLocalRotation (Variables|Default|GetAzimuth%20Gimbal) (Math|Rotator|MakeRotator 0.0 0.0 (* AxisValue (Utilities|Time|GetWorldDeltaSeconds) 1e+02)) false false))

(event Input|AxisEvents|InputAxisAimElevation
  (params (AxisValue :type Float%20%28single-precision%29))
  (Transformation|AddLocalRotation (Variables|Default|GetSpringArm) (Math|Rotator|MakeRotator 0.0 (* AxisValue (Utilities|Time|GetWorldDeltaSeconds) 1e+02) 0.0) false false))

(event Input|GamepadEvents|GamepadLeftX
  (params (AxisValue :type Float%20%28single-precision%29))
  (Class|TankMovementComponent|IntendMoveRight (Variables|Default|GetTankMovement) AxisValue))

(event Input|GamepadEvents|GamepadLeftY
  (params (AxisValue :type Float%20%28single-precision%29))
  (Class|TankMovementComponent|IntendMoveForward (Variables|Default|GetTankMovement) AxisValue))

(event Input|GamepadEvents|GamepadFaceButtonBottom
  (params (Key :type Key%20Structure))
  (:Pressed
    (Class|TankAimingComponent|Fire (Variables|Default|GetTankAiming))))

(fn ConstructionScript
  (bind _meshes (Variables|Default|GetMeshes))
  (for _index (range 0 (- (Spline|GetNumberOfSplinePoints (Variables|Default|GetSpline1)) 1))
    (bind _returnvalue (AddComponent|AddSplineMeshComponent false))
    (Transformation|AttachComponentToComponent _returnvalue (Variables|Default|GetSpline1) "None" "KeepRelative" "KeepRelative" "KeepRelative" true)
    (bind _returnvalue_2 (Utilities|Array|Add _meshes _returnvalue))
    (SplineMesh|SetStartandEnd _returnvalue (Math|Vector|MakeVector (.x (Spline|GetLocationatSplinePoint (Variables|Default|GetSpline1) _index "Local")) (.y (Spline|GetLocationatSplinePoint (Variables|Default|GetSpline1) _index "Local")) (.z (Spline|GetLocationatSplinePoint (Variables|Default|GetSpline1) _index "Local"))) (Spline|GetTangentatSplinePoint (Variables|Default|GetSpline1) _index "Local") (.Location (Spline|GetLocationandTangentatSplinePoint (Variables|Default|GetSpline1) (+ _index 1) "Local")) (.Tangent (Spline|GetLocationandTangentatSplinePoint (Variables|Default|GetSpline1) (+ _index 1) "Local")) true :!class /Script/Engine.SplineMeshComponent)
    (Collision|SetCollisionEnabled _returnvalue "QueryOnly")
    (switch int (Math|Integer|%(Integer) _returnvalue_2 2)
      (:0
        (Rendering|Material|SetMaterial (Utilities|Array|Get(acopy) _meshes _returnvalue_2) 0 "/Engine/EngineDebugMaterials/VertexColorViewMode_RedOnly.VertexColorViewMode_RedOnly")))))

(fn InitializeHealthBarWidget
  (bind _asbp_health_bar (Utilities|Casting|CastToBP_HealthBar (UserInterface|GetUserWidgetObject (Variables|Default|GetWidget))))
  (Variables|/Game/UI/BP_HealthBar.BP_HealthBar_C|SetMyTank _asbp_health_bar self)
  (return))

(fn Movetreads
  (bind _spline1 (Variables|Default|GetSpline1))
  (for _index (range 0 (- (Spline|GetNumberOfSplinePoints (Variables|Default|GetSpline1)) 1))
    (Development|PrintString "Hello")
    (SplineMesh|SetStartandEnd (Utilities|Array|Get(acopy) (Variables|Default|GetMeshes) _index) (Spline|GetLocationatSplinePoint _spline1 (+ _index 1) "Local") (Spline|GetTangentatSplinePoint _spline1 (+ _index 1) "Local") (Spline|GetLocationatSplinePoint _spline1 (+ _index 2) "Local") (Spline|GetTangentatSplinePoint _spline1 (+ _index 2) "Local") true :!class /Script/Engine.SplineMeshComponent)
    (Development|PrintString (Utilities|String|Append (Utilities|String|ToString(Integer) _index) (Utilities|String|ToString(Vector) (Transformation|GetWorldLocation (Utilities|Array|Get(acopy) (Variables|Default|GetMeshes) _index)))))))