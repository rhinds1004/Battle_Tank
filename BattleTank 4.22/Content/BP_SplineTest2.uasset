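; Test actor that lays out a vehicle tread as spline mesh segments along Spline1.
; The construction script adds query-only segments at fixed distance steps, giving every other one a debug red material.
; BeginPlay advances a wrapped offset from left-track velocity and repositions each segment along the spline, forcing roll to 180 where the right vector flips.
; This runs only once because Tick is empty, and several point-based experiments are left unconnected.
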(event EventBeginPlay
  (bind _spline1 (Variables|Default|GetSpline1))
  (bind _returnvalue (Spline|GetSplineLength _spline1))
  (Variables|Default|SetTreadMeshOffsetLeft (.Remainder (Math|Float|Division(WholeandRemainder) (+ (Variables|Default|GetTreadMeshOffsetLeft) (* (Variables|Default|GetTrackLeftLinVel) (Utilities|Time|GetWorldDeltaSeconds))) (Spline|GetSplineLength (Variables|Default|GetSpline1)))))
  (for _index (range 0 (- (Utilities|Array|Length (Variables|Default|GetNewVar_0)) 1))
    (Transformation|SetRelativeLocationAndRotation (Utilities|Array|Get(acopy) (Variables|Default|GetNewVar_0) _index) (Spline|GetLocationatDistanceAlongSpline _spline1 (Math|Float|SelectFloat (+ _returnvalue (.Remainder (Math|Float|Division(WholeandRemainder) (+ (* _index (/ _returnvalue 69.0)) (Variables|Default|GetTreadMeshOffsetLeft)) _returnvalue))) (.Remainder (Math|Float|Division(WholeandRemainder) (+ (* _index (/ _returnvalue 69.0)) (Variables|Default|GetTreadMeshOffsetLeft)) _returnvalue)) (< (.Remainder (Math|Float|Division(WholeandRemainder) (+ (* _index (/ _returnvalue 69.0)) (Variables|Default|GetTreadMeshOffsetLeft)) _returnvalue)) 0.0)) "Local") (Math|Rotator|MakeRotator (Math|Float|SelectFloat 1.8e+02 (.roll (Spline|GetRotationatDistanceAlongSpline _spline1 (Math|Float|SelectFloat (+ _returnvalue (.Remainder (Math|Float|Division(WholeandRemainder) (+ (* _index (/ _returnvalue 69.0)) (Variables|Default|GetTreadMeshOffsetLeft)) _returnvalue))) (.Remainder (Math|Float|Division(WholeandRemainder) (+ (* _index (/ _returnvalue 69.0)) (Variables|Default|GetTreadMeshOffsetLeft)) _returnvalue)) (< (.Remainder (Math|Float|Division(WholeandRemainder) (+ (* _index (/ _returnvalue 69.0)) (Variables|Default|GetTreadMeshOffsetLeft)) _returnvalue)) 0.0)) "Local")) (< (.y (Class|SplineComponent|GetRightVectoratDistanceAlongSpline _spline1 (Math|Float|SelectFloat (+ _returnvalue (.Remainder (Math|Float|Division(WholeandRemainder) (+ (* _index (/ _returnvalue 69.0)) (Variables|Default|GetTreadMeshOffsetLeft)) _returnvalue))) (.Remainder (Math|Float|Division(WholeandRemainder) (+ (* _index (/ _returnvalue 69.0)) (Variables|Default|GetTreadMeshOffsetLeft)) _returnvalue)) (< (.Remainder (Math|Float|Division(WholeandRemainder) (+ (* _index (/ _returnvalue 69.0)) (Variables|Default|GetTreadMeshOffsetLeft)) _returnvalue)) 0.0)) "Local")) 0.0)) (.pitch (Spline|GetRotationatDistanceAlongSpline _spline1 (Math|Float|SelectFloat (+ _returnvalue (.Remainder (Math|Float|Division(WholeandRemainder) (+ (* _index (/ _returnvalue 69.0)) (Variables|Default|GetTreadMeshOffsetLeft)) _returnvalue))) (.Remainder (Math|Float|Division(WholeandRemainder) (+ (* _index (/ _returnvalue 69.0)) (Variables|Default|GetTreadMeshOffsetLeft)) _returnvalue)) (< (.Remainder (Math|Float|Division(WholeandRemainder) (+ (* _index (/ _returnvalue 69.0)) (Variables|Default|GetTreadMeshOffsetLeft)) _returnvalue)) 0.0)) "Local")) (.yaw (Spline|GetRotationatDistanceAlongSpline _spline1 (Math|Float|SelectFloat (+ _returnvalue (.Remainder (Math|Float|Division(WholeandRemainder) (+ (* _index (/ _returnvalue 69.0)) (Variables|Default|GetTreadMeshOffsetLeft)) _returnvalue))) (.Remainder (Math|Float|Division(WholeandRemainder) (+ (* _index (/ _returnvalue 69.0)) (Variables|Default|GetTreadMeshOffsetLeft)) _returnvalue)) (< (.Remainder (Math|Float|Division(WholeandRemainder) (+ (* _index (/ _returnvalue 69.0)) (Variables|Default|GetTreadMeshOffsetLeft)) _returnvalue)) 0.0)) "Local"))) false false)
    (SplineMesh|UpdateMesh (Utilities|Array|Get(acopy) (Variables|Default|GetNewVar_0) _index))))

(event Collision|EventActorBeginOverlap
  (params (OtherActor :type Actor%20Object%20Reference)))

(event EventTick
  (params (DeltaSeconds :type Float%20%28single-precision%29)))

(fn ConstructionScript
  (bind _spline1 (Variables|Default|GetSpline1))
  (bind _spline1_2 (Variables|Default|GetSpline1))
  (bind _returnvalue (Spline|GetSplineLength _spline1_2))
  (while (<= (Variables|Default|GetCurrDist) _returnvalue)
    (bind _returnvalue_2 (AddComponent|AddSplineMeshComponent false))
    (Transformation|AttachComponentToComponent _returnvalue_2 (Variables|Default|GetSpline1) "None" "KeepRelative" "KeepRelative" "KeepRelative" true)
    (bind _returnvalue_3 (Utilities|Array|Add (Variables|Default|GetNewVar_0) _returnvalue_2))
    (SplineMesh|SetStartandEnd _returnvalue_2 (Spline|GetLocationatDistanceAlongSpline (Variables|Default|GetSpline1) (Variables|Default|GetPrevDist) "Local") (Spline|GetTangentatDistanceAlongSpline _spline1 (Variables|Default|GetPrevDist) "Local") (Spline|GetLocationatDistanceAlongSpline (Variables|Default|GetSpline1) (Variables|Default|GetCurrDist) "Local") (Spline|GetTangentatDistanceAlongSpline _spline1 (Variables|Default|GetCurrDist) "Local") true :!class /Script/Engine.SplineMeshComponent)
    (Collision|SetCollisionEnabled _returnvalue_2 "QueryOnly")
    (Variables|Default|SetPrevDist (Variables|Default|GetCurrDist))
    (Variables|Default|SetCurrDist (+ (Variables|Default|GetCurrDist) 2e+01))
    (switch int (Math|Integer|%(Integer) _returnvalue_3 2)
      (:0
        (Rendering|Material|SetMaterial (Utilities|Array|Get(acopy) (Variables|Default|GetNewVar_0) _returnvalue_3) 0 "/Engine/EngineDebugMaterials/VertexColorViewMode_RedOnly.VertexColorViewMode_RedOnly"))))
  (if (not (Math|Float|NearlyEqual(Float) (- _returnvalue (Variables|Default|GetCurrDist)) 0.0 1e-06))
    (bind _returnvalue_4 (AddComponent|AddSplineMeshComponent false))
    (Transformation|AttachComponentToComponent _returnvalue_4 (Variables|Default|GetSpline1) "None" "KeepRelative" "KeepRelative" "KeepRelative" true)
    (bind _returnvalue_5 (Utilities|Array|Add (Variables|Default|GetNewVar_0) _returnvalue_4))
    (SplineMesh|SetStartandEnd _returnvalue_4 (Spline|GetLocationatDistanceAlongSpline (Variables|Default|GetSpline1) (Variables|Default|GetPrevDist) "Local") (Spline|GetTangentatDistanceAlongSpline _spline1 (Variables|Default|GetPrevDist) "Local") (Spline|GetLocationatDistanceAlongSpline (Variables|Default|GetSpline1) (Variables|Default|GetCurrDist) "Local") (Spline|GetTangentatDistanceAlongSpline _spline1 (Variables|Default|GetCurrDist) "Local") true :!class /Script/Engine.SplineMeshComponent)
    (Collision|SetCollisionEnabled _returnvalue_4 "QueryOnly")
    (Variables|Default|SetPrevDist (Variables|Default|GetCurrDist))
    (Variables|Default|SetCurrDist (+ (Variables|Default|GetCurrDist) 2e+01))
    (switch int (Math|Integer|%(Integer) _returnvalue_5 2)
      (:0
        (Rendering|Material|SetMaterial (Utilities|Array|Get(acopy) (Variables|Default|GetNewVar_0) _returnvalue_5) 0 "/Engine/EngineDebugMaterials/VertexColorViewMode_RedOnly.VertexColorViewMode_RedOnly")))))